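; BP_EMPPlatform is a platform that emits an EMP pulse whenever an actor begins overlapping it.
; The pulse gathers electric objects within EMPRadius through GetAllElectricInRadius, passing itself as source, and sends each an EMPPulseMessage.
; A green debug sphere shows the radius, drawn from the construction script and redrawn every tick.
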(event EventBeginPlay)

(event Collision|EventActorBeginOverlap
  (params (OtherActor :type Actor%20Object%20Reference))
  (CallFunction|SendEmpPulse))

(event EventTick
  (params (DeltaSeconds :type Float%20%28single-precision%29))
  (CallFunction|DrawSphere))

(fn ConstructionScript
  (CallFunction|DrawSphere))

(fn DrawSphere
  (Rendering|Debug|DrawDebugSphere (Transformation|GetActorLocation self) (Variables|Default|GetEMPRadius) 12 "(R=0.300843,G=1.000000,B=0.286705,A=1.000000)" 0.0 1.0))

(fn SendEmpPulse
  (bind _electricdevices (CallFunction|GetAllElectricinRadius (Variables|Default|GetEMPRadius) self))
  (for _array_element _electricdevices
    (Class|BPIElectricDevice|EMPPulse(Message) _array_element)))