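; BP_WallSconce is a wall sconce light with configurable brightness, color and inner and outer cone angles.
; Its construction script calls InitializeLight to apply those settings to the SconceLight component, then applies the IsLit state.
; UpdateLight stores the on/off state in IsLit and toggles the light component's visibility without propagating to its children.
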(fn ConstructionScript
  (CallFunction|InitializeLight)
  (CallFunction|UpdateLight (Variables|Default|GetIsLit)))

(fn UpdateLight
  (params (IsOn :type Boolean))
  (bind _output_get (Variables|Default|SetIsLit IsOn))
  (Rendering|SetVisibility (Variables|Default|GetSconceLight) _output_get false))

(fn InitializeLight
  (Rendering|Components|Light|SetIntensity (Variables|Default|GetSconceLight) (Variables|Light|GetBrightness))
  (Rendering|Components|Light|SetLightColor (Variables|Default|GetSconceLight) (Variables|Light|GetColor) true)
  (Rendering|Lighting|SetInnerConeAngle (Variables|Default|GetSconceLight) (Variables|Light|GetInner%20Cone%20Angle))
  (Rendering|Lighting|SetOuterConeAngle (Variables|Default|GetSconceLight) (Variables|Light|GetOuter%20Cone%20Angle)))