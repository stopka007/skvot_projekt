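; Base NPC character that takes damage, dies as a ragdoll and can be taken down.
; Damage goes to SkvtHealthComponent and plays a hit montage; its death signal disables movement, starts mesh physics and destroys the actor on a timer.
; TakeDownArea overlaps toggle CanTakeDown on the overlapping BP_SkvtBaseChar.
; The Takedown event bypasses health, disabling movement and collision, playing a neck-break montage, then destroying the NPC after a delay.
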(event OnComponentBeginOverlap(TakeDownArea)
  (params (OverlappedComponent :type Primitive%20Component%20Object%20Reference) (OtherActor :type Actor%20Object%20Reference) (OtherComp :type Primitive%20Component%20Object%20Reference) (OtherBodyIndex :type Integer) (bFromSweep :type Boolean) (SweepResult :type Hit%20Result%20Structure%20%28by%20ref%29))
  ;[0 0 0] Takedown
  (bind _asbp_skvt_base_char (Utilities|Casting|CastToBP_SkvtBaseChar OtherActor))
  (Variables|/Game/Skvt/Characters/BP_SkvtBaseChar.BP_SkvtBaseChar_C|SetCanTakeDown? _asbp_skvt_base_char true))

(event SignalCharacterDeath(SkvtHealthComponent)
  (CallFunction|TriggerDeath))

(event OnComponentEndOverlap(TakeDownArea)
  (params (OverlappedComponent :type Primitive%20Component%20Object%20Reference) (OtherActor :type Actor%20Object%20Reference) (OtherComp :type Primitive%20Component%20Object%20Reference) (OtherBodyIndex :type Integer))
  ;[0 0 0] Takedown
  (bind _asbp_skvt_base_char (Utilities|Casting|CastToBP_SkvtBaseChar OtherActor))
  (Variables|/Game/Skvt/Characters/BP_SkvtBaseChar.BP_SkvtBaseChar_C|SetCanTakeDown? _asbp_skvt_base_char false))

(event Custom|Takedown
  ;[0 0 0] Takedown
  (Pawn|Components|CharacterMovement|DisableMovement (Variables|Character|GetCharacterMovement))
  (Collision|SetActorEnableCollision false)
  (Animation|PlayAnimMontage "/Game/Skvt/Characters/Animations/Attacks/AM_Hit_BreakNeckLonger.AM_Hit_BreakNeckLonger" 1.0 "None")
  (Utilities|FlowControl|Delay 3.5)
  (Actor|DestroyActor))

(event EventBeginPlay)

(event Collision|EventActorBeginOverlap
  (params (OtherActor :type Actor%20Object%20Reference)))

(event EventTick
  (params (DeltaSeconds :type Float%20%28single-precision%29)))

(event Game|Damage|EventAnyDamage
  (params (Damage :type Float%20%28single-precision%29) (DamageType :type Damage%20Type%20Object%20Reference) (InstigatedBy :type Controller%20Object%20Reference) (DamageCauser :type Actor%20Object%20Reference))
  (Default|ProcessDamage (Variables|Default|GetSkvtHealthComponent) Damage)
  (Animation|PlayAnimMontage "/Game/Skvt/Characters/Animations/Attacks/AM_Hit_punch.AM_Hit_punch" 1.0 "None"))

(fn ConstructionScript)

(fn TriggerDeath
  (Physics|SetSimulatePhysics (Variables|Character|GetMesh) true)
  (Pawn|Components|CharacterMovement|DisableMovement (Variables|Character|GetCharacterMovement))
  (Utilities|Time|SetTimerbyFunctionName 0 "FinalizeDeath" 5.0))

(fn FinalizeDeath
  (Actor|DestroyActor))